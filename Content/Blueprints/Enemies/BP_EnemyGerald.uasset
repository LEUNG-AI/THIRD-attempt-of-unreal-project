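; BP_EnemyGerald is a sprite-based enemy that walks constantly along the world X axis.
; BeginPlay picks a random MoveRight flag and mirrors the sprite when it is true, while Tick feeds movement input that resolves to negative X for either value.
; The capsule hit event is empty, and EnemyDied calls the parent logic before destroying the actor.
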(event OnComponentHit(CapsuleComponent)
  (params (HitComponent :type Primitive%20Component%20Object%20Reference) (OtherActor :type Actor%20Object%20Reference) (OtherComp :type Primitive%20Component%20Object%20Reference) (NormalImpulse :type Vector :default "0, 0, 0") (Hit :type Hit%20Result%20Structure%20%28by%20ref%29)))

(event EventBeginPlay
  (bind _sprite (Variables|Default|GetSprite))
  (bind _returnvalue (Transformation|GetWorldScale _sprite))
  (Variables|Default|SetMove%20Right (Math|Random|RandomBool))
  (Transformation|SetWorldScale3D (Variables|Default|GetSprite) (Math|Vector|MakeVector (* (.x _returnvalue) (select (Variables|Default|GetMove%20Right) -1.0 1.0)) (.y _returnvalue) (.z _returnvalue))))

(event EventTick
  (params (DeltaSeconds :type Float%20%28single-precision%29))
  (Pawn|Input|AddMovementInput "1.000000, 0, 0" (select (Variables|Default|GetMove%20Right) -1.0 -1.0) false))

(fn ConstructionScript
  (|CallParentFunction))

(fn EnemyDied
  (|CallParentFunction)
  (Actor|DestroyActor))